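; BP_Nest is an actor that spawns a Turtle and acts as its nest.
; On BeginPlay it spawns the Turtle high above its own location, ignoring collisions, and passes itself to it through SetNest.
; GetTarget exposes the TargetPoint for other objects to query.
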(event `self.ReceiveBeginPlay`
  (bind _returnvalue (`|SpawnActorFromClass` (`self.Turtle`) (`KismetMathLibrary.MakeTransform` (+ (`self.K2_GetActorLocation`) (0.0 0.0 1000.0))) "AlwaysSpawn" "OverrideRootScale" null null))
  (`/Game/Crow/Actors/Pawns/BP_Crow.SetNest` _returnvalue self))

(event `self.ReceiveTick`
  (params (DeltaSeconds :type "Float (single-precision)")))

(fn `GetTarget`
  (returns (Target :type "/Game/Crow/Actors/BP_Target Object Reference"))
  (return (`self.TargetPoint`)))

(fn `UserConstructionScript`
  (`parent.UserConstructionScript`))